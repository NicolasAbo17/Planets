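; Planet actor that switches gravitational pull on the first-person space character as it enters and leaves the atmosphere.
; Overlaps on the Atmosphere component count only for components tagged Body, whose owner is cast to BP_FirstPersonSpace.
; Entering starts that character's gravitational force with this planet as the source and leaving stops it, each printing a debug string.
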(event `self.Atmosphere.OnComponentBeginOverlap`
  (params (OverlappedComponent :type "PrimitiveComponent Object Reference") (OtherActor :type "Actor Object Reference") (OtherComp :type "PrimitiveComponent Object Reference") (OtherBodyIndex :type Integer) (bFromSweep :type Boolean) (SweepResult :type "HitResult Structure (by ref)"))
  (if (`ActorComponent.ComponentHasTag` OtherComp "Body")
    (bind _asbp_first_person_space (cast `/Game/Space/Blueprints/BP_FirstPersonSpace` OtherActor))
    (`/Game/Space/Blueprints/BP_FirstPersonSpace.Start Gravitational Force` _asbp_first_person_space self)
    (`KismetSystemLibrary.PrintString` "Gravity")))

(event `self.Atmosphere.OnComponentEndOverlap`
  (params (OverlappedComponent :type "PrimitiveComponent Object Reference") (OtherActor :type "Actor Object Reference") (OtherComp :type "PrimitiveComponent Object Reference") (OtherBodyIndex :type Integer))
  (if (`ActorComponent.ComponentHasTag` OtherComp "Body")
    (bind _asbp_first_person_space (cast `/Game/Space/Blueprints/BP_FirstPersonSpace` OtherActor))
    (`/Game/Space/Blueprints/BP_FirstPersonSpace.StopGravitationalForce` _asbp_first_person_space)
    (`KismetSystemLibrary.PrintString` "NoGravity")))

(fn `UserConstructionScript`)